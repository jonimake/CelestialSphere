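; Actor that builds a procedural celestial sphere of stars from a star data table.
; Setting the UpdateMesh flag makes the Construction Script reset it and rebuild once, acting as a button.
; The rebuild synchronously loads the soft-referenced table, copies its rows into Stars, then passes them to ConvertCoordinates and BuildMesh.
; The event graph holds no active logic.
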(fn `UserConstructionScript`
  (locals (stars :type "Array of Star Structure") (DebugStars :type "Array of Star Structure"))
  (bind _stardatatable (`self.StarDataTable`))
  (if (`self.UpdateMesh?`)
    (set `self.UpdateMesh?` false)
    (`|ExecutionSequence`
      (:`then_0`
        (`KismetSystemLibrary.LoadAsset_Blocking` _stardatatable)
        (bind _returnvalue (`self.GetRowData` (`|ConvertAsset` _stardatatable)))
        (set `local.stars` _returnvalue))
      (:`then_1`
        (`self.ConvertCoordinates` (`local.stars`)))
      (:`then_2`
        (`self.BuildMesh` (`local.stars`))))))